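; BP_Pickup is a placeable pickup spawner whose collected state is recorded in the game instance by ActorID.
; Shortly after BeginPlay it destroys itself if already recorded, otherwise hides its Sphere and spawns either a random pick from three object classes or a manual class there.
; When the third-person character overlaps its Er component, it records the ID as destroyed and removes itself, leaving the spawned actor untouched.
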(event OnComponentBeginOverlap(er)
  (params (OverlappedComponent :type Primitive%20Component%20Object%20Reference) (OtherActor :type Actor%20Object%20Reference) (OtherComp :type Primitive%20Component%20Object%20Reference) (OtherBodyIndex :type Integer) (bFromSweep :type Boolean) (SweepResult :type Hit%20Result%20Structure%20%28by%20ref%29))
  (Utilities|Casting|CastToBP_ThirdPersonCharacter OtherActor)
  (CallFunction|PickUp)
  (Actor|DestroyActor))

(event Custom|PickUp
  (bind _asmy_game_instance (Utilities|Casting|CastToMyGameInstance (Game|GetGameInstance)))
  (Default|DestoryItem _asmy_game_instance (Variables|Default|GetActor%20ID)))

(event Custom|SetArrayRan
  (bind _output_get (Variables|Default|SetRandomItemArray (Utilities|Array|MakeArray (Variables|Default|GetObjectA) (Variables|Default|GetObjectC) (Variables|Default|GetObjectB)))))

(event EventBeginPlay
  (CallFunction|SetArrayRan)
  (Utilities|FlowControl|Delay 0.2)
  (bind _asmy_game_instance (Utilities|Casting|CastToMyGameInstance (Game|GetGameInstance)))
  (bind _destoryedalready (Default|CheckifAlreadyDestoryed _asmy_game_instance (Variables|Default|GetActor%20ID)))
  (if _destoryedalready
    (Actor|DestroyActor)
    (else
      (Utilities|FlowControl|Delay 0.5)
      (if true
        (Development|SetHiddeninGame (Variables|Default|GetSphere) true false))
      (if (Variables|Default|GetIsUsingRandomObject)
        (Game|SpawnActorfromClass (Utilities|Array|Get(acopy) (stale Custom|SetArrayRan _output_get) (Math|Random|RandomInteger 3)) (Math|Conversions|ToTransform(Vector) (Transformation|GetWorldLocation (Variables|Default|GetSphere))) "Undefined" 0 0)
        (else
          (Game|SpawnActorfromClass (Variables|Default|GetManualObject) (Math|Conversions|ToTransform(Vector) (Transformation|GetWorldLocation (Variables|Default|GetSphere))) "Undefined" 0 0))))))

(fn ConstructionScript
  (bind _output_get (Variables|Default|SetRandomItemArray (Utilities|Array|MakeArray (Variables|Default|GetObjectA) (Variables|Default|GetObjectC) (Variables|Default|GetObjectB)))))