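; Spawner actor that spawns actors at four aim points when BP_ThirdPersonCharacter overlaps its sphere trigger.
; With IsUsingRandomArray on, it picks random classes from four, filling one pair of aims per overlap, gated by BridgeStartingPair and SpawningNotDone until both pairs are done.
; Otherwise every overlap spawns ClassA through ClassD at their matching aims, with no guard against repeats.
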(event OnComponentBeginOverlap(Sphere1)
  (params (OverlappedComponent :type Primitive%20Component%20Object%20Reference) (OtherActor :type Actor%20Object%20Reference) (OtherComp :type Primitive%20Component%20Object%20Reference) (OtherBodyIndex :type Integer) (bFromSweep :type Boolean) (SweepResult :type Hit%20Result%20Structure%20%28by%20ref%29))
  (bind _arrayofclasses (Variables|Default|GetArrayOfClasses))
  (bind _outitem (Utilities|Array|Random _arrayofclasses))
  (Utilities|Casting|CastToBP_ThirdPersonCharacter OtherActor)
  (if (Variables|Default|GetIsUsingRandomArray)
    (if (Variables|Default|GetSpawningNotDone)
      (if (Variables|Default|GetBridgeStartingPair)
        (Game|SpawnActorfromClass _outitem (Transformation|GetWorldTransform (Variables|Aims|GetSpawnAim1)) "Undefined" 0 0)
        (Game|SpawnActorfromClass _outitem (Transformation|GetWorldTransform (Variables|Aims|GetSpawnAim2)) "Undefined" 0 0)
        (Variables|Default|SetBridgeStartingPair false)
        (else
          (Game|SpawnActorfromClass _outitem (Transformation|GetWorldTransform (Variables|Aims|GetSpawnAim3)) "Undefined" 0 0)
          (Game|SpawnActorfromClass _outitem (Transformation|GetWorldTransform (Variables|Aims|GetSpawnAim4)) "Undefined" 0 0)
          (Variables|Default|SetSpawningNotDone false))))
    (else
      (Game|SpawnActorfromClass (Variables|Default|GetClass%20A) (Transformation|GetWorldTransform (Variables|Aims|GetSpawnAim1)) "Undefined" 0 0)
      (Game|SpawnActorfromClass (Variables|Default|GetClass%20B) (Transformation|GetWorldTransform (Variables|Aims|GetSpawnAim2)) "Undefined" 0 0)
      (Game|SpawnActorfromClass (Variables|Default|GetClass%20C) (Transformation|GetWorldTransform (Variables|Aims|GetSpawnAim3)) "Undefined" 0 0)
      (Game|SpawnActorfromClass (Variables|Default|GetClass%20D) (Transformation|GetWorldTransform (Variables|Aims|GetSpawnAim4)) "Undefined" 0 0))))

(event EventBeginPlay
  (Variables|Default|SetArrayOfClasses (Utilities|Array|MakeArray (Variables|Classes|GetClassA) (Variables|Classes|GetClassB) (Variables|Classes|GetClassC) (Variables|Classes|GetClassD)))
  (bind _output_get (Variables|Aims|SetSpawnAims (Utilities|Array|MakeArray (Variables|Aims|GetSpawnAim1) (Variables|Aims|GetSpawnAim2) (Variables|Aims|GetSpawnAim3) (Variables|Aims|GetSpawnAim4)))))

(event Collision|EventActorBeginOverlap
  (params (OtherActor :type Actor%20Object%20Reference)))

(event EventTick
  (params (DeltaSeconds :type Float%20%28single-precision%29)))

(fn ConstructionScript)