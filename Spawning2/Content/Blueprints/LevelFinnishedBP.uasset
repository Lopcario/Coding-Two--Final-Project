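; Level-finish trigger that declares a win and resets the current level when BP_ThirdPersonCharacter overlaps its Sphere.
; On overlap it deletes the save game slot and overwrites DestroyedActors on MyGameInstance with its own DestroyedActors value.
; It then prints a delayed on-screen countdown and reopens the current level by name.
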(event OnComponentBeginOverlap(Sphere)
  (params (OverlappedComponent :type Primitive%20Component%20Object%20Reference) (OtherActor :type Actor%20Object%20Reference) (OtherComp :type Primitive%20Component%20Object%20Reference) (OtherBodyIndex :type Integer) (bFromSweep :type Boolean) (SweepResult :type Hit%20Result%20Structure%20%28by%20ref%29))
  (Utilities|Casting|CastToBP_ThirdPersonCharacter OtherActor)
  (Development|PrintString "You win! Level will now reset...")
  (SaveGame|DeleteGameinSlot (Variables|Default|GetSlot%20Name1))
  (bind _returnvalue (Game|GetCurrentLevelName true))
  (Utilities|FlowControl|Sequence
    (:then_0
      (bind _asmy_game_instance (Utilities|Casting|CastToMyGameInstance (Game|GetGameInstance)))
      (Variables|/Game/Blueprints/MyGameInstance.MyGameInstance_C|SetDestroyedActors _asmy_game_instance (Variables|Default|GetDestroyedActors)))
    (:then_1
      (Development|PrintString "Restarting level...")
      (Utilities|FlowControl|Delay 2.0)
      (Development|PrintString "3...")
      (Utilities|FlowControl|Delay 1.5)
      (Development|PrintString "2...")
      (Utilities|FlowControl|Delay 1.5)
      (Development|PrintString "1...")
      (Utilities|FlowControl|Delay 1.5)
      (Game|OpenLevel(byName) (Utilities|String|StringToName _returnvalue)))))

(event EventBeginPlay)

(event Collision|EventActorBeginOverlap
  (params (OtherActor :type Actor%20Object%20Reference)))

(event EventTick
  (params (DeltaSeconds :type Float%20%28single-precision%29)))

(fn ConstructionScript)