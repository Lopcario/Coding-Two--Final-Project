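; BP_ToolTipTrigger is a trigger actor, in a deprecated folder, that shows tooltip text on the player's UI.
; When BP_ThirdPersonCharacter overlaps it, it passes VolumeText to the character and enters a DoOnce that plays the PlayerUI tooltip animation.
; After a delay it flags the display as done.
; If ShouldDisplayAgain is set, Tick then resets the DoOnce, clearing PlayerIsInVolume every frame, so its in-volume check always passes.
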(event Collision|EventActorBeginOverlap
  (params (OtherActor :type Actor%20Object%20Reference))
  (bind _asbp_third_person_character (Utilities|Casting|CastToBP_ThirdPersonCharacter OtherActor))
  (Variables|Default|SetbPlayerIsInVolume true)
  (Variables|/Game/ThirdPerson/Blueprints/BP_ThirdPersonCharacter.BP_ThirdPersonCharacter_C|SetToolTipToDisplay _asbp_third_person_character (Variables|ToolTipSettings|GetVolumeText))
  (Utilities|FlowControl|DoOnce false
    (:Completed
      (UserInterface|Animation|PlayAnimation (Variables|/Game/ThirdPerson/Blueprints/BP_ThirdPersonCharacter.BP_ThirdPersonCharacter_C|GetPlayer%20UI _asbp_third_person_character) (Variables|/Game/Blueprints/depricated/BP_PlayerUI_Jade.BP_PlayerUI_Jade_C|GetToolTipAnimation (Variables|/Game/ThirdPerson/Blueprints/BP_ThirdPersonCharacter.BP_ThirdPersonCharacter_C|GetPlayer%20UI _asbp_third_person_character)) 0.0 1 "Forward" (Variables|ToolTipSettings|GetAnimationPlaybackSpeed) false)
      (Utilities|FlowControl|Delay (Variables|ToolTipSettings|GetAnimation%20Reset%20Delay))
      (Variables|Default|SetbPlayerIsInVolume false)
      (Variables|Default|SetbIsDoneDisplaying true))))

(event EventTick
  (params (DeltaSeconds :type Float%20%28single-precision%29))
  (if (Variables|ToolTipSettings|GetbShouldDisplayAgain?)
    (bind _output_get (Variables|Default|SetbPlayerIsInVolume false))
    (if (and (not _output_get) (Variables|Default|GetbIsDoneDisplaying))
      (Variables|Default|SetbIsDoneDisplaying false)
      (Utilities|FlowControl|DoOnce false) ; enters at Reset
    )))

(fn ConstructionScript)