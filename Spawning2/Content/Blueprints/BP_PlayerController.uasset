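; Player controller that persists the world seed and the list of destroyed actors in a MySaveGame slot.
; SaveGame loads or creates the save and copies in the GameInstance's destroyed-actor list; LoadGame copies it back, retrying on a short delay until the GameInstance reference is valid.
; SetWorldSeed seeds a new save only when none exists, but the following SaveGame call replaces that object, losing the seed.
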(event Custom|SetWorldSeed
  (bind _returnvalue (SaveGame|DoesSaveGameExist (Variables|Default|GetSlot%20Name)))
  (if (not _returnvalue)
    (bind _returnvalue_2 (SaveGame|CreateSaveGameObject "/Game/Blueprints/MySaveGame.MySaveGame_C"))
    (Variables|Default|SetSave%20Game%20REF _returnvalue_2)
    (Variables|/Game/Blueprints/MySaveGame.MySaveGame_C|SetSeed _returnvalue_2 (Variables|Default|GetINT))
    (bind _asmy_save_game (Utilities|Casting|CastToMySaveGame (Variables|Default|GetSave%20Game%20REF)))
    (Development|PrintString (Utilities|String|ToString(Integer) (Variables|/Game/Blueprints/MySaveGame.MySaveGame_C|GetSeed _asmy_save_game)))
    (CallFunction|SaveGame)))

(event Custom|Load%20Game
  ;[1 1 1] Load destoryed actors
  (Utilities|IsValid (Variables|Default|GetGame%20Instance%20REF) :!label _label
    (:Is%20Valid
      (bind _returnvalue (SaveGame|LoadGamefromSlot (Variables|Default|GetSlot%20Name)))
      (bind _asmy_save_game (Utilities|Casting|CastToMySaveGame _returnvalue))
      (bind _output_get (Variables|Default|SetSave%20Game%20REF _asmy_save_game))
      (Variables|/Game/Blueprints/MyGameInstance.MyGameInstance_C|SetDestroyedActors (Variables|Default|GetGame%20Instance%20REF) (Variables|/Game/Blueprints/MySaveGame.MySaveGame_C|GetDestoryedActors _output_get)))
    (:Is%20Not%20Valid
      (Utilities|FlowControl|Delay 0.2)
      (goto _label))))

(event Custom|Save%20Game
  ;[1 1 1] save list of destoryed actors
  (bind _returnvalue (SaveGame|DoesSaveGameExist (Variables|Default|GetSlot%20Name)))
  (if _returnvalue
    (bind _returnvalue_2 (SaveGame|LoadGamefromSlot (Variables|Default|GetSlot%20Name)))
    (bind _asmy_save_game (Utilities|Casting|CastToMySaveGame _returnvalue_2))
    (Variables|Default|SetSave%20Game%20REF _asmy_save_game)
    (else
      (bind _returnvalue_3 (SaveGame|CreateSaveGameObject "/Game/Blueprints/MySaveGame.MySaveGame_C"))
      (bind _asmy_save_game_2 (Utilities|Casting|CastToMySaveGame _returnvalue_3))
      (Variables|Default|SetSave%20Game%20REF _asmy_save_game_2)))
  (Variables|/Game/Blueprints/MySaveGame.MySaveGame_C|SetDestoryedActors (Variables|Default|GetSave%20Game%20REF) (Variables|/Game/Blueprints/MyGameInstance.MyGameInstance_C|GetDestroyedActors (Variables|Default|GetGame%20Instance%20REF)))
  (SaveGame|SaveGametoSlot (Variables|Default|GetSave%20Game%20REF) (Variables|Default|GetSlot%20Name)))

(event EventTick
  (params (DeltaSeconds :type Float%20%28single-precision%29)))

(event EventBeginPlay
  (bind _asmy_game_instance (Utilities|Casting|CastToMyGameInstance (Game|GetGameInstance)))
  (Variables|Default|SetGame%20Instance%20REF _asmy_game_instance))

(fn ConstructionScript)